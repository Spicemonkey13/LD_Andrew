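; Melee zombie enemy that damages and knocks back whatever its hitbox overlaps.
; A target counts as in range when it overlaps that same hitbox.
; The damage event applies point damage to every overlapping actor without filtering, along the zombie's forward vector.
; Overlapping Characters are also launched in that direction by the knockback strength, overriding horizontal velocity only.
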(event `/Game/GameConent/Enemies/BI_Enemies.Enemy_DoDamage`
  (for _array_element (`PrimitiveComponent.GetOverlappingActors` (`self.Hitbox`) null)
    (`GameplayStatics.ApplyPointDamage` _array_element (`self.Damage`) (`self.GetActorForwardVector`) (`GameplayStatics.MakeHitResult` false) null self)
    (bind _ascharacter (cast `Character` _array_element))
    (`self.LaunchCharacter` _ascharacter (* (`self.GetActorForwardVector`) (`self.KnockbackStrength`)) true false)))

(fn `Enemy_CheckTargetInRange`
  (params (Target :type "Actor Object Reference"))
  (returns (bSuccess :type Boolean))
  (return (`KismetArrayLibrary.Array_Contains` (`PrimitiveComponent.GetOverlappingActors` (`self.Hitbox`) null) Target)))

(fn `UserConstructionScript`
  (`parent.UserConstructionScript`))